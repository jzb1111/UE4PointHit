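; Demo actor for custom Blueprint functions that fills a transform array and spawns child actors, named as bunnies, at those transforms.
; BeginPlay calls CallOnCalcLocation, defined outside this file, then SpawnBunny.
; AddToTransformArray appends an unrotated, unit-scale transform built from the LocationX/Y/Z variables, with no caller in these graphs.
; SpawnBunny adds a child actor component per array entry, branching between first and later elements.
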(event EventBeginPlay
  (Default|CallOnCalcLocation)
  (CallFunction|SpawnBunny))

(event Collision|EventActorBeginOverlap
  (params (OtherActor :type Actor%20Object%20Reference)))

(event EventTick
  (params (DeltaSeconds :type Float%20%28single-precision%29)))

(fn ConstructionScript)

(fn SpawnBunny
  (for (_array_element _array_index) (Variables|Default|Gettransform)
    (if (> _array_index 0)
      (AddComponent|AddChildActorComponent false _array_element)
      (else
        (AddComponent|AddChildActorComponent false _array_element)))))

(fn AddtoTransformArray
  (Utilities|Array|Add (Variables|Default|Gettransform) (Math|Transform|MakeTransform (Math|Vector|MakeVector (Variables|Default|GetLocationX) (Variables|Default|GetLocationY) (Variables|Default|GetLocationZ)))))